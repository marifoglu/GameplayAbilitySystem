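; BP_FlamePiller is a flame pillar actor that makes its FireLight flicker continuously from BeginPlay.
; ChooseTimeline randomly starts one of two flame intensity timelines, each scaling BaseIntensity by its curve to set the light's intensity.
; When a timeline finishes, it calls ChooseTimeline again, forming an endless, varied flicker loop without using Tick.
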(event Custom|StartLight_2
  (bind _lightintensity (Timeline|FlameIntensity_2 PlayFromStart)
    (:Update
      (Rendering|Components|Light|SetIntensity (Variables|Default|GetFireLight) (* _lightintensity (Variables|Default|GetBaseIntensity))))
    (:Finished
      (CallFunction|ChooseTimeline))))

(event Custom|StartLight_1
  (bind _lightintensity (Timeline|FlameIntensity_1 PlayFromStart)
    (:Update
      (Rendering|Components|Light|SetIntensity (Variables|Default|GetFireLight) (* _lightintensity (Variables|Default|GetBaseIntensity))))
    (:Finished
      (CallFunction|ChooseTimeline))))

(event Custom|ChooseTimeline
  (switch int (Math|Random|RandomIntegerinRange 0 1)
    (:Default
      (CallFunction|StartLight2 :!label _label))
    (:0
      (CallFunction|StartLight1))
    (:1
      (goto _label))))

(event EventBeginPlay
  (CallFunction|ChooseTimeline))

(fn ConstructionScript)